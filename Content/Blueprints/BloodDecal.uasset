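; BloodDecal is an actor that displays a randomized blood splatter decal.
; On BeginPlay it picks a random material from the BloodSplatters array and applies it to its Decal component.
; It then randomizes the actor's yaw over a full turn while keeping pitch and roll, so each splatter varies in both pattern and orientation.
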(event EventBeginPlay
  (bind _returnvalue (Transformation|GetActorRotation))
  (Rendering|Components|Decal|SetDecalMaterial (Variables|Decal|GetDecal) (Utilities|Array|Get(acopy) (Variables|Default|GetBloodSplatters) (Math|Random|RandomIntegerinRange 0 (- (Utilities|Array|Length (Variables|Default|GetBloodSplatters)) 1))))
  (Transformation|SetActorRotation (Math|Rotator|MakeRotator (.roll _returnvalue) (.pitch _returnvalue) (Math|Random|RandomFloatinRange 0.0 3.6e+02))))

(fn ConstructionScript)