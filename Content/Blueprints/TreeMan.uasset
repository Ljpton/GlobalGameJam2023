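; TreeMan is a tree actor that the player can topple once every Root actor in the level is destroyed.
; On BeginPlay it counts the Roots and binds to each one's OnRootDestroyed event to decrement RootsAlive.
; Each destruction updates a TreeWidget with the remaining count or a final prompt, creating the widget while RootUIVisible is false, though nothing here sets that flag.
; Player overlap at zero roots calls Die, enabling physics on the tree.
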(event Custom|OnRootDestroyed
  (Development|PrintString "Root Destroyed!")
  (Variables|Default|SetRootsAlive (- (Variables|Default|GetRootsAlive) 1))
  (if (Variables|Default|GetRootUIVisible)
    _
    (else
      (bind _returnvalue (UserInterface|CreateWidget "/Game/2D/Widgets/TreeWidget.TreeWidget_C"))
      (bind _output_get (Variables|Default|SetTreeUI _returnvalue))
      (UserInterface|Viewport|AddtoViewport _output_get 0)))
  (Rendering|Components|TextRender|SetText (Variables|/Game/2D/Widgets/TreeWidget.TreeWidget_C|GetRootsValue (Variables|Default|GetTreeUI)) (Utilities|Text|ToText(String) (Utilities|String|SelectString "Get rid of that tree now!" (Utilities|String|ToString(Integer) (Variables|Default|GetRootsAlive)) (<= (Variables|Default|GetRootsAlive) 0)))))

(event Custom|Die
  (Physics|SetSimulatePhysics (Variables|Default|GetTree) true)
  (Development|PrintString "Simulate"))

(event EventBeginPlay
  (bind _outactors (Actor|GetAllActorsOfClass "/Game/Blueprints/Root.Root_C"))
  (bind _output_get (Variables|Default|SetRootCount (Utilities|Array|Length _outactors)))
  (Variables|Default|SetRootsAlive _output_get)
  (for _array_element _outactors
    (EventDispatchers|BindEventtoOnRootDestroyed _array_element (delegate Custom|OnRootDestroyed))))

(event Collision|EventActorBeginOverlap
  (params (OtherActor :type Actor%20Object%20Reference))
  (Development|PrintString "Hello")
  (if (and (== OtherActor (Game|Player|GetPlayerPawn 0)) (<= (Variables|Default|GetRootsAlive) 0))
    (CallFunction|Die)))

(fn ConstructionScript)